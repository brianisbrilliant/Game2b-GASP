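; BP_Lever is an interactable lever that the sandbox character reaches for with right-hand IK and toggles with F.
; Sphere overlap caches the character's AnimBP, enables input and fades IK alpha in on a timeline, reversing it on exit.
; F drives a FlipFlop that plays or reverses a second timeline, slerping the Handle's relative location.
; During movement, the IK target follows the StaticMesh location while the character remains in range.
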(event `self.ReceiveBeginPlay`)

(event `self.SphereCollision.OnComponentBeginOverlap`
  (params (OverlappedComponent :type "PrimitiveComponent Object Reference") (OtherActor :type "Actor Object Reference") (OtherComp :type "PrimitiveComponent Object Reference") (OtherBodyIndex :type Integer) (bFromSweep :type Boolean) (SweepResult :type "HitResult Structure (by ref)"))
  (bind _assandbox_character_cmc2 (cast `/Game/SandboxCharacter_CMC2` OtherActor))
  (bind _assandbox_character_cmc_abp2 (cast `/Game/SandboxCharacter_CMC_ABP2` (`SkeletalMeshComponent.GetAnimInstance` (`Character.Mesh` _assandbox_character_cmc2)))) ; Get a reference to the specific AnimBP\nthat we're editing.
  (bind _output_get (set `self.AnimBP` _assandbox_character_cmc_abp2)) ; Save this variable for later.
  (set `self.TouchingButton` true)
  (`self.EnableInput` (`GameplayStatics.GetPlayerController` 0))
  (set `/Game/SandboxCharacter_CMC_ABP2.RightHandIKTarget` (`SceneComponent.K2_GetComponentLocation` (`self.Handle`)) _output_get)
  (bind (_direction _newtrack_0) (`Timeline|Timeline` :!via `PlayFromStart` :!label _label)
    (:`Update`
      (set `/Game/SandboxCharacter_CMC_ABP2.RightHandIKAlpha` _newtrack_0 (`self.AnimBP`)))
    (:`Finished`
      (`self.UpdateHandPosition`))))

(event `self.SphereCollision.OnComponentEndOverlap`
  (params (OverlappedComponent :type "PrimitiveComponent Object Reference") (OtherActor :type "Actor Object Reference") (OtherComp :type "PrimitiveComponent Object Reference") (OtherBodyIndex :type Integer))
  (`self.DisableInput` (`GameplayStatics.GetPlayerController` 0))
  (set `self.TouchingButton` false)
  (goto _label :!via `Reverse`))

(event `UpdateHandPosition`
  (if (`self.TouchingButton`)
    (bind _animbp (`self.AnimBP`)
      (:`then`
        (set `/Game/SandboxCharacter_CMC_ABP2.RightHandIKTarget` (`SceneComponent.K2_GetComponentLocation` (`self.StaticMesh`)) _animbp))
      (:`else`))))

(event `Key|F`
  (params (Key :type "Key Structure"))
  (:`Pressed`
    (`self.Move Lever`)))

(event `Move Lever`
  (`/Engine/EditorBlueprintResources/StandardMacros.FlipFlop`
    (:`A`
      (bind (_direction _newtrack_0) (`Timeline|Timeline_0` :!label _label_2)
        (:`Update`
          (`SceneComponent.K2_SetRelativeLocation` (`self.Handle`) (`KismetMathLibrary.Vector_SlerpNormals` (0.0 0.0 100.0) (0.0 10.0 100.0) _newtrack_0) false false)
          (`self.UpdateHandPosition`))))
    (:`B`
      (goto _label_2 :!via `Reverse`))))

(fn `UserConstructionScript`)